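; Player controller that steers the player's ship pawn, fetching pawn and mesh references through an interface message on BeginPlay and showing the mouse cursor.
; W, touch or P_MoveForward_1 starts continuous forward movement, while A and D strafe only while held.
; Looping timers, using the latest tick delta as interval, add movement input along the mesh's axes.
; GPauseGame pauses forward movement and teleports the pawn to a fixed position.
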(event `self.ReceiveBeginPlay`
  ;[1 1 1] BeginPlay
  (set `self.bShowMouseCursor` true)
  (bind (_playerpawn _shipmesh) (message `/Game/Blueprints/MainPlayer/BPI_Player.GetReferences` (`GameplayStatics.GetPlayerPawn` 0)))
  (set `self.Player Pawn` _playerpawn)
  (set `self.Ship Mesh` _shipmesh))

(event `self.ReceiveTick`
  (params (DeltaSeconds :type "Float (single-precision)"))
  ;[1 1 1] Event Tick
  (set `self.Delta Seconds` DeltaSeconds))

(event `/Game/Blueprints/MainPlayer/BPI_Controller.G_PauseGame`
  (`KismetSystemLibrary.K2_PauseTimerHandle` (`self.timer_MoveForward`))
  (`self.K2_TeleportTo` :`self` (`self.Player Pawn`) :`DestLocation` (1500.0 -600.0 250.0)))

(event `P_MoveForward_1`
  (`self.E_StartForwardMovement`))

(event `E_StartForwardMovement`
  ;[1 1 1] Forward Movement
  (bind _returnvalue (`KismetSystemLibrary.K2_SetTimerDelegate` (delegate `E_MoveForward`) (`self.Delta Seconds`) true))
  (set `self.timer_MoveForward` _returnvalue))

(event `Key|W`
  (params (Key :type "Key Structure"))
  ;[1 1 1] W_Keyboard
  (:`Pressed`
    (`self.E_StartForwardMovement` :!label _label)))

(event `Key|D`
  (params (Key :type "Key Structure"))
  ;[1 1 1] Comment
  (:`Pressed`
    (bind _returnvalue (`KismetSystemLibrary.K2_SetTimerDelegate` (delegate `E_MoveRight`) (`self.Delta Seconds`) true))
    (set `self.timer_MoveRight` _returnvalue))
  (:`Released`
    (`KismetSystemLibrary.K2_PauseTimerHandle` (`self.timer_MoveRight`))))

(event `InputTouch`
  (params (Location :type "Vector Structure") (FingerIndex :type "ETouchIndex Enum"))
  ;[1 1 1] W_Keyboard
  (:`Pressed`
    (goto _label)))

(event `E_MoveRight`
  ;[1 1 1] Comment
  (`Pawn.AddMovementInput` (`self.Player Pawn`) (`SceneComponent.GetRightVector` (`self.Ship Mesh`)) 20.0 false))

(event `E_MoveForward`
  ;[1 1 1] Forward Movement
  (`Pawn.AddMovementInput` (`self.Player Pawn`) (`SceneComponent.GetForwardVector` (`self.Ship Mesh`)) 10.0 false))

(event `Key|A`
  (params (Key :type "Key Structure"))
  ;[1 1 1] Comment
  (:`Pressed`
    (bind _returnvalue (`KismetSystemLibrary.K2_SetTimerDelegate` (delegate `E_MoveLeft`) (`self.Delta Seconds`) true))
    (set `self.timer_MoveLeft` _returnvalue))
  (:`Released`
    (`KismetSystemLibrary.K2_PauseTimerHandle` (`self.timer_MoveLeft`))))

(event `E_MoveLeft`
  ;[1 1 1] Comment
  (`Pawn.AddMovementInput` (`self.Player Pawn`) (`SceneComponent.GetRightVector` (`self.Ship Mesh`)) -20.0 false))

(fn `UserConstructionScript`)